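; BP_Exploding_Trap is a side-scroller trap that explodes when the player character touches it.
; An overlap on its collision sphere, filtered by a cast to 2DSideScrollerCharacter, spawns a BP_Kunai_Trap at the world transform of each of its five arrow components.
; It then plays an explosion particle effect and sound at the sprite's position and destroys itself.
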(event `self.Sphere_Collision.OnComponentBeginOverlap`
  (params (OverlappedComponent :type "PrimitiveComponent Object Reference") (OtherActor :type "Actor Object Reference") (OtherComp :type "PrimitiveComponent Object Reference") (OtherBodyIndex :type Integer) (bFromSweep :type Boolean) (SweepResult :type "HitResult Structure (by ref)"))
  (bind _papersprite (`self.PaperSprite`))
  (bind _returnvalue (`SceneComponent.K2_GetComponentLocation` _papersprite))
  (cast `/Game/Character/2DSideScrollerCharacter` OtherActor)
  (for _array_element (`|MakeArray` (`self.Arrow1`) (`self.Arrow2`) (`self.Arrow3`) (`self.Arrow4`) (`self.Arrow`))
    (`|SpawnActorFromClass` "/Game/Items/Kunai/BP_Kunai_Trap.BP_Kunai_Trap_C" (`SceneComponent.K2_GetComponentToWorld` _array_element) "Undefined" "OverrideRootScale" null null))
  (`GameplayStatics.SpawnEmitterAtLocation` "/Game/StarterContent/Particles/P_Explosion.P_Explosion" _returnvalue (`SceneComponent.K2_GetComponentRotation` _papersprite))
  (`GameplayStatics.PlaySoundAtLocation` "/Game/StarterContent/Audio/Explosion01.Explosion01" _returnvalue (struct) 1.0 1.0 0.0 null null null)
  (`self.K2_DestroyActor`))

(fn `UserConstructionScript`)